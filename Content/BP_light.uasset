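; BP_light is an actor that flashes its point light a set number of times when play begins.
; BeginPlay runs a self-looping DoN limited by FlashCount, with each pass waiting FlashSpeed before toggling PointLight1's visibility.
; After each toggle, a single-pass for loop increments ScreenCount, prints it to screen and feeds back into the DoN.
; Overlap, Tick and the construction script are empty.
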(event `self.ReceiveBeginPlay`
  (`/Engine/EditorBlueprintResources/StandardMacros.Do N` (`KismetMathLibrary.FTrunc` (`self.FlashCount`)) :!label _label
    (:`Exit`
      (`KismetSystemLibrary.Delay` (`self.FlashSpeed`))
      (`SceneComponent.ToggleVisibility` (`self.PointLight1`) false)
      (for _ (range 1)
        (bind _result (`/Engine/EditorBlueprintResources/StandardMacros.IncrementInt` (`self.Screen Count`))
          (:`  `
            (`KismetSystemLibrary.PrintString` (`KismetStringLibrary.Conv_IntToString` _result))
            (goto _label)))))))

(event `self.ReceiveActorBeginOverlap`
  (params (OtherActor :type "Actor Object Reference")))

(event `self.ReceiveTick`
  (params (DeltaSeconds :type "Float (single-precision)")))

(fn `UserConstructionScript`)